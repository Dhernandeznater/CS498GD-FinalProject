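; Flame hazard actor that damages the player on a repeating off, ready and flaming cycle.
; Three functions chain through timers from BeginPlay, each showing its flipbook and hiding the other two.
; A sphere overlap passes the hazard's location to Player_BP's HandleEnemyDamage, only while FlameState is true.
; Damage fires only on overlap begin, so a player already inside when the flames ignite is not hit.
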(event `self.ReceiveBeginPlay`
  (`self.flamesOff`))

(event `self.Sphere.OnComponentBeginOverlap`
  (params (OverlappedComponent :type "PrimitiveComponent Object Reference") (OtherActor :type "Actor Object Reference") (OtherComp :type "PrimitiveComponent Object Reference") (OtherBodyIndex :type Integer) (bFromSweep :type Boolean) (SweepResult :type "HitResult Structure (by ref)"))
  (if (`self.flameState`)
    (bind _asplayer_bp (cast `/Game/Blueprints/Player_BP` OtherActor))
    (`/Game/Blueprints/Player_BP.HandleEnemyDamage` _asplayer_bp (`self.K2_GetActorLocation`))))

(fn `flamesOff`
  (set `self.flameState` false)
  (`KismetSystemLibrary.K2_SetTimer` null "flamesReady" 3.0)
  (`SceneComponent.SetVisibility` (`self.ReadyFlipbook`) false false)
  (`SceneComponent.SetVisibility` (`self.FlamingFlipbook`) false false)
  (`SceneComponent.SetVisibility` (`self.OffFlipbook`) true false))

(fn `flamesOn`
  (`SceneComponent.SetVisibility` (`self.ReadyFlipbook`) false false)
  (`SceneComponent.SetVisibility` (`self.FlamingFlipbook`) true false)
  (`SceneComponent.SetVisibility` (`self.OffFlipbook`) false false)
  (set `self.flameState` true)
  (`KismetSystemLibrary.K2_SetTimer` null "flamesOff" 3.0))

(fn `flamesReady`
  (`KismetSystemLibrary.K2_SetTimer` null "flamesOn" 1.0)
  (`SceneComponent.SetVisibility` (`self.ReadyFlipbook`) true false)
  (`SceneComponent.SetVisibility` (`self.FlamingFlipbook`) false false)
  (`SceneComponent.SetVisibility` (`self.OffFlipbook`) false false))

(fn `UserConstructionScript`)