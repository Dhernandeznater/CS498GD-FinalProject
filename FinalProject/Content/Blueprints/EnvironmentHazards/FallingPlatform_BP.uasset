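; FallingPlatform_BP is a hazard platform that drops after the player hits it.
; A Box hit from Player_BP sets the flipbook play rate and starts a short timer calling setFalling, which switches to the off flipbook.
; Tick then accumulates velocity from FallAccel and moves the actor along Z with a swept SetActorLocation.
; Only acceleration is scaled by delta time, so fall speed depends on frame rate.
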(event `self.ReceiveTick`
  (params (DeltaSeconds :type "Float (single-precision)"))
  (if (`self.falling`)
    (bind _output_get (set `self.fallVelocity` (+ (* (`self.fallAccel`) DeltaSeconds) (`self.fallVelocity`))))
    (`self.K2_SetActorLocation` (+ (`KismetMathLibrary.MakeVector` 0.0 0.0 _output_get) (`self.K2_GetActorLocation`)) true)))

(event `self.Box.OnComponentHit`
  (params (HitComponent :type "PrimitiveComponent Object Reference") (OtherActor :type "Actor Object Reference") (OtherComp :type "PrimitiveComponent Object Reference") (NormalImpulse :type "Vector Structure") (Hit :type "HitResult Structure (by ref)"))
  (cast `/Game/Blueprints/Player_BP` OtherActor)
  (`PaperFlipbookComponent.SetPlayRate` (`self.PaperFlipbook`) 0.5)
  (`KismetSystemLibrary.K2_SetTimer` null "setFalling" 0.6))

(fn `setFalling`
  (set `self.falling` true)
  (`PaperFlipbookComponent.SetFlipbook` (`self.PaperFlipbook`) "/Game/Art/Traps/Flipbooks/FallingPlatform_Off_Flipbook.FallingPlatform_Off_Flipbook"))

(fn `UserConstructionScript`)