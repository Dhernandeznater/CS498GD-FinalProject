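; WalkerEnemyChar_BP is a walker enemy character that paces back and forth along world X and can be killed through its KillTop component.
; Tick applies movement input from Speed and the Direction boolean, which a looping timer flips at SwapSpeed plus a random offset chosen at BeginPlay.
; When Player_BP overlaps KillTop, the walker destroys itself and calls HandleEnemyKill.
; Capsule hits call the player's HandleEnemyDamage with the walker's location.
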(event `self.ReceiveBeginPlay`
  (bind _output_get (set `self.randomVariance` (`KismetMathLibrary.RandomFloatInRange` 0.0 3.0)))
  (`KismetSystemLibrary.K2_SetTimer` null "swapDirection" (+ _output_get (`self.swapSpeed`)) true))

(event `self.ReceiveTick`
  (params (DeltaSeconds :type "Float (single-precision)"))
  (`self.AddMovementInput` (1.0 0.0 0.0) (* (`KismetMathLibrary.MapRangeClamped` (`KismetMathLibrary.Conv_BoolToDouble` (`self.direction`)) 0.0 1.0 -1.0 1.0) (`self.Speed`))))

(event `self.KillTop.OnComponentBeginOverlap`
  (params (OverlappedComponent :type "PrimitiveComponent Object Reference") (OtherActor :type "Actor Object Reference") (OtherComp :type "PrimitiveComponent Object Reference") (OtherBodyIndex :type Integer) (bFromSweep :type Boolean) (SweepResult :type "HitResult Structure (by ref)"))
  (bind _asplayer_bp (cast `/Game/Blueprints/Player_BP` OtherActor))
  (`self.K2_DestroyActor`)
  (`/Game/Blueprints/Player_BP.HandleEnemyKill` _asplayer_bp))

(event `self.CapsuleComponent.OnComponentHit`
  (params (HitComponent :type "PrimitiveComponent Object Reference") (OtherActor :type "Actor Object Reference") (OtherComp :type "PrimitiveComponent Object Reference") (NormalImpulse :type "Vector Structure") (Hit :type "HitResult Structure (by ref)"))
  (bind _asplayer_bp (cast `/Game/Blueprints/Player_BP` OtherActor))
  (`/Game/Blueprints/Player_BP.HandleEnemyDamage` _asplayer_bp (`self.K2_GetActorLocation`)))

(fn `SwapDirection`
  (set `self.direction` (not (`self.direction`))))

(fn `UserConstructionScript`)