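; Flying bird enemy with a flipbook sprite that patrols along X and can be killed by the player.
; A looping, randomly offset timer reverses direction, while Tick adds movement input with a sine-wave vertical bob.
; Player overlap with KillTop plays the hit flipbook, notifies the player and expires the bird shortly after; capsule hits damage the player unless it is dead.
; SwapDirection sets identical scale in both branches, so it never mirrors the sprite.
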(event `self.ReceiveBeginPlay`
  (bind _output_get (set `self.randomVariance` (`KismetMathLibrary.RandomFloatInRange` 0.0 3.0)))
  (`CharacterMovementComponent.SetMovementMode` (`self.CharacterMovement`) "MOVE_Flying" 0)
  (`KismetSystemLibrary.K2_SetTimer` null "swapDirection" (+ _output_get (`self.swapSpeed`)) true))

(event `self.ReceiveTick`
  (params (DeltaSeconds :type "Float (single-precision)"))
  (`self.AddMovementInput` (`KismetMathLibrary.MakeVector` (`KismetMathLibrary.MapRangeClamped` (`KismetMathLibrary.Conv_BoolToDouble` (`self.direction`)) 0.0 1.0 -1.0 1.0) 0.0 (`KismetMathLibrary.Sin` (+ (`self.randomVariance`) (`GameplayStatics.GetUnpausedTimeSeconds`)))) (`self.Speed`)))

(event `self.KillTop.OnComponentBeginOverlap`
  (params (OverlappedComponent :type "PrimitiveComponent Object Reference") (OtherActor :type "Actor Object Reference") (OtherComp :type "PrimitiveComponent Object Reference") (OtherBodyIndex :type Integer) (bFromSweep :type Boolean) (SweepResult :type "HitResult Structure (by ref)"))
  (bind _asplayer_bp (cast `/Game/Blueprints/Player_BP` OtherActor))
  (`self.SetLifeSpan` 0.2)
  (`/Game/Blueprints/Player_BP.HandleEnemyKill` _asplayer_bp)
  (`PaperFlipbookComponent.SetFlipbook` (`self.Sprite`) "/Game/Art/Sprites/Enemies/Flipbooks/Bird_Hit_Flipbook.Bird_Hit_Flipbook")
  (`PaperFlipbookComponent.SetPlayRate` (`self.Sprite`) 1.0)
  (set `self.dead` true))

(event `self.CapsuleComponent.OnComponentHit`
  (params (HitComponent :type "PrimitiveComponent Object Reference") (OtherActor :type "Actor Object Reference") (OtherComp :type "PrimitiveComponent Object Reference") (NormalImpulse :type "Vector Structure") (Hit :type "HitResult Structure (by ref)"))
  (bind _asplayer_bp (cast `/Game/Blueprints/Player_BP` OtherActor))
  (if (not (`self.dead`))
    (`/Game/Blueprints/Player_BP.HandleEnemyDamage` _asplayer_bp (`self.K2_GetActorLocation`))))

(fn `SwapDirection`
  (bind _output_get (set `self.direction` (not (`self.direction`))))
  (if _output_get
    (`SceneComponent.SetRelativeScale3D` (`self.Sprite`) (1.0 1.0 1.0))
    (else
      (`SceneComponent.SetRelativeScale3D` (`self.Sprite`) (1.0 1.0 1.0)))))

(fn `UserConstructionScript`)