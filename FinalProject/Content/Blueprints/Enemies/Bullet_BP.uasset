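; Bullet_BP is an enemy projectile that flies in a straight line toward the player and damages them on contact.
; On BeginPlay it sets its lifespan and locks a direction to the player pawn's current location, so it does not home.
; Tick moves it with a swept location update scaled by Speed.
; Sphere overlaps with Player_BP call HandleEnemyDamage with the bullet's location, without destroying the bullet.
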(event `self.ReceiveBeginPlay`
  (`self.SetLifeSpan` (`self.lifeSpan`))
  (set `self.direction` (`KismetMathLibrary.GetDirectionUnitVector` (`self.K2_GetActorLocation`) (`self.K2_GetActorLocation` (`GameplayStatics.GetPlayerPawn` 0)))))

(event `self.ReceiveTick`
  (params (DeltaSeconds :type "Float (single-precision)"))
  (`self.K2_SetActorLocation` (+ (`self.K2_GetActorLocation`) (* (`self.direction`) (* DeltaSeconds (`self.speed`)))) true))

(event `self.Sphere.OnComponentBeginOverlap`
  (params (OverlappedComponent :type "PrimitiveComponent Object Reference") (OtherActor :type "Actor Object Reference") (OtherComp :type "PrimitiveComponent Object Reference") (OtherBodyIndex :type Integer) (bFromSweep :type Boolean) (SweepResult :type "HitResult Structure (by ref)"))
  (bind _asplayer_bp (cast `/Game/Blueprints/Player_BP` OtherActor))
  (`/Game/Blueprints/Player_BP.HandleEnemyDamage` _asplayer_bp (`self.K2_GetActorLocation`)))

(fn `UserConstructionScript`)