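; Angry Pig walker enemy that patrols along the X axis and speeds toward the player inside an aggro radius.
; A looping timer with a random offset reverses patrol direction, while Tick picks walk or run flipbooks and faces the sprite toward the player only during a chase.
; Overlapping KillTop kills it and notifies Player_BP.
; Capsule hits while alive damage the player.
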(event `self.ReceiveBeginPlay`
  (bind _output_get (set `self.randomVariance` (`KismetMathLibrary.RandomFloatInRange` 0.0 3.0)))
  (`KismetSystemLibrary.K2_SetTimer` null "swapDirection" (+ _output_get (`self.swapSpeed`)) true))

(event `self.ReceiveTick`
  (params (DeltaSeconds :type "Float (single-precision)"))
  (bind _returnvalue (`self.K2_GetActorLocation`))
  (bind _returnvalue_2 (`self.K2_GetActorLocation` (`GameplayStatics.GetPlayerPawn` 0)))
  (bind _x (.x (`KismetMathLibrary.GetDirectionUnitVector` _returnvalue _returnvalue_2)))
  (if (not (`self.dead`))
    ;[1 1 1] Aggro
    (`/Engine/EditorBlueprintResources/StandardMacros.CompareFloat` (`self.agroRadius`) (`KismetMathLibrary.Vector_Distance` _returnvalue_2 _returnvalue)
      (:`>`
        (`self.AddMovementInput` (1.0 0.0 0.0) (* (`self.agroSpeed`) _x))
        (`SceneComponent.SetRelativeScale3D` (`self.Sprite`) (`KismetMathLibrary.MakeVector` (* -1.0 (`KismetMathLibrary.SignOfFloat` _x)) 1.0 1.0))
        (`PaperFlipbookComponent.SetFlipbook` (`self.Sprite`) "/Game/Art/Sprites/Enemies/Flipbooks/Angry_Pig_Run_Flipbook.Angry_Pig_Run_Flipbook")
        (`PaperFlipbookComponent.SetPlayRate` (`self.Sprite`) 2.0))
      (:`==`
        ;[1 1 1] Patrol
        (`self.AddMovementInput` (1.0 0.0 0.0) (* (`KismetMathLibrary.MapRangeClamped` (`KismetMathLibrary.Conv_BoolToDouble` (`self.direction`)) 0.0 1.0 -1.0 1.0) (`self.Speed`)) :!label _label)
        (`PaperFlipbookComponent.SetFlipbook` (`self.Sprite`) "/Game/Art/Sprites/Enemies/Flipbooks/Angry_Pig_Walk_Flipbook.Angry_Pig_Walk_Flipbook")
        (`PaperFlipbookComponent.SetPlayRate` (`self.Sprite`) 1.0))
      (:`<`
        (goto _label)))))

(event `self.KillTop.OnComponentBeginOverlap`
  (params (OverlappedComponent :type "PrimitiveComponent Object Reference") (OtherActor :type "Actor Object Reference") (OtherComp :type "PrimitiveComponent Object Reference") (OtherBodyIndex :type Integer) (bFromSweep :type Boolean) (SweepResult :type "HitResult Structure (by ref)"))
  (bind _asplayer_bp (cast `/Game/Blueprints/Player_BP` OtherActor))
  (`self.SetLifeSpan` 0.2)
  (`/Game/Blueprints/Player_BP.HandleEnemyKill` _asplayer_bp)
  (`PaperFlipbookComponent.SetFlipbook` (`self.Sprite`) "/Game/Art/Sprites/Enemies/Flipbooks/Angry_Pig_Hit_Flipbook.Angry_Pig_Hit_Flipbook")
  (`PaperFlipbookComponent.SetPlayRate` (`self.Sprite`) 1.0)
  (set `self.dead` true))

(event `self.CapsuleComponent.OnComponentHit`
  (params (HitComponent :type "PrimitiveComponent Object Reference") (OtherActor :type "Actor Object Reference") (OtherComp :type "PrimitiveComponent Object Reference") (NormalImpulse :type "Vector Structure") (Hit :type "HitResult Structure (by ref)"))
  (bind _asplayer_bp (cast `/Game/Blueprints/Player_BP` OtherActor))
  (if (not (`self.dead`))
    (`/Game/Blueprints/Player_BP.HandleEnemyDamage` _asplayer_bp (`self.K2_GetActorLocation`))))

(fn `SwapDirection`
  (bind _output_get (set `self.direction` (not (`self.direction`))))
  (if _output_get
    (`SceneComponent.SetRelativeScale3D` (`self.Sprite`) (1.0 1.0 1.0))
    (else
      (`SceneComponent.SetRelativeScale3D` (`self.Sprite`) (1.0 1.0 1.0)))))

(fn `UserConstructionScript`)