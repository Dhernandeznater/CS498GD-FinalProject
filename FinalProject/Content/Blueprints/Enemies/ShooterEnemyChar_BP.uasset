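; Shooter enemy character, a flipbook-animated plant that periodically attacks the player within its aggro radius.
; A looping timer with a random offset runs the range check, turns the sprite toward the player and triggers delayed timers that spawn an actor at KillTop and restore idle.
; Player overlap with KillTop kills it, showing a hit flipbook before it expires.
; Capsule hits damage the player while it is alive.
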(event `self.ReceiveBeginPlay`
  (bind _output_get (set `self.randomVariance` (`KismetMathLibrary.RandomFloatInRange` 0.0 1.0)))
  (`KismetSystemLibrary.K2_SetTimer` null "attemptShoot" (+ _output_get (`self.shootTime`)) true))

(event `self.KillTop.OnComponentBeginOverlap`
  (params (OverlappedComponent :type "PrimitiveComponent Object Reference") (OtherActor :type "Actor Object Reference") (OtherComp :type "PrimitiveComponent Object Reference") (OtherBodyIndex :type Integer) (bFromSweep :type Boolean) (SweepResult :type "HitResult Structure (by ref)"))
  (bind _asplayer_bp (cast `/Game/Blueprints/Player_BP` OtherActor))
  (`self.SetLifeSpan` 0.2)
  (`/Game/Blueprints/Player_BP.HandleEnemyKill` _asplayer_bp)
  (`PaperFlipbookComponent.SetFlipbook` (`self.Sprite`) "/Game/Art/Sprites/Enemies/Flipbooks/Plant_Hit_Flipbook.Plant_Hit_Flipbook")
  (`PaperFlipbookComponent.SetPlayRate` (`self.Sprite`) 1.0)
  (set `self.dead` true))

(event `self.CapsuleComponent.OnComponentHit`
  (params (HitComponent :type "PrimitiveComponent Object Reference") (OtherActor :type "Actor Object Reference") (OtherComp :type "PrimitiveComponent Object Reference") (NormalImpulse :type "Vector Structure") (Hit :type "HitResult Structure (by ref)"))
  (bind _asplayer_bp (cast `/Game/Blueprints/Player_BP` OtherActor))
  (if (not (`self.dead`))
    (`/Game/Blueprints/Player_BP.HandleEnemyDamage` _asplayer_bp (`self.K2_GetActorLocation`))))

(fn `attemptShoot`
  (bind _returnvalue (`self.K2_GetActorLocation`))
  (bind _returnvalue_2 (`self.K2_GetActorLocation` (`GameplayStatics.GetPlayerPawn` 0)))
  (`/Engine/EditorBlueprintResources/StandardMacros.CompareFloat` (`self.agroRadius`) (`KismetMathLibrary.Vector_Distance` _returnvalue_2 _returnvalue)
    (:`>`
      (`SceneComponent.SetRelativeScale3D` (`self.Sprite`) (`KismetMathLibrary.MakeVector` (* -1.0 (`KismetMathLibrary.SignOfFloat` (.x (`KismetMathLibrary.GetDirectionUnitVector` _returnvalue _returnvalue_2)))) 1.0 1.0))
      (`PaperFlipbookComponent.SetFlipbook` (`self.Sprite`) "/Game/Art/Sprites/Enemies/Flipbooks/Plant_Attack_Flipbook.Plant_Attack_Flipbook")
      (`PaperFlipbookComponent.SetPlayRate` (`self.Sprite`) 1.0)
      (`KismetSystemLibrary.K2_SetTimer` null "endShootAnim" 0.5)
      (`KismetSystemLibrary.K2_SetTimer` null "shoot" 0.3))))

(fn `endShootAnim`
  (`PaperFlipbookComponent.SetFlipbook` (`self.Sprite`) "/Game/Art/Sprites/Enemies/Flipbooks/Plant_Idle_Flipbook.Plant_Idle_Flipbook")
  (`PaperFlipbookComponent.SetPlayRate` (`self.Sprite`) 1.0))

(fn `shoot`
  (`|SpawnActorFromClass` "/Game/Blueprints/Enemies/Bullet_BP.Bullet_BP_C" (`SceneComponent.K2_GetComponentToWorld` (`self.KillTop`)) "Undefined" "OverrideRootScale" null null))

(fn `UserConstructionScript`)