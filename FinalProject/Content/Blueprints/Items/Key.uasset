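; Key pickup actor with a Paper2D sprite that the player collects by touching it.
; On overlap with Player_BP, it passes the sprite's first component tag to CollectKey, so the tag identifies the key.
; A delayed countdown loop then steps the sprite's alpha down before destroying the actor; an untagged key is destroyed without being collected.
; FadeToBlack is an unused empty stub, and a debug "Hello" prints on any overlap.
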(event `self.ReceiveActorBeginOverlap`
  (params (OtherActor :type "Actor Object Reference"))
  (bind _componenttags (`ActorComponent.ComponentTags` (`self.PaperSprite`)))
  ;[1 1 1] Fade on collid with player
  (`KismetSystemLibrary.PrintString` "Hello")
  (bind _asplayer_bp (cast `/Game/Blueprints/Player_BP` OtherActor))
  (if (> (`KismetArrayLibrary.Array_Length` _componenttags) 0)
    (`/Game/Blueprints/Player_BP.Collect Key` _asplayer_bp (`KismetStringLibrary.Conv_NameToString` (`|GetArrayItem` _componenttags)))
    (for _index (range 10 1)
      (`KismetSystemLibrary.Delay` 0.1)
      (`PaperSpriteComponent.SetSpriteColor` (`self.PaperSprite`) (make `LinearColor` 0.0 0.0 0.0 (/ (`KismetMathLibrary.Conv_IntToDouble` _index) 10.0)))))
  (`self.K2_DestroyActor`))

(fn `FadeToBlack`
  (while (> 0.0 0.0)
    _))

(fn `UserConstructionScript`)